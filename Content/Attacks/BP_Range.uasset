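; BP_Range is the player's ranged attack projectile, which damages the enemy it hits.
; On BeginPlay it places itself 80 units in front of player 0, yawed -90 degrees from the player's facing.
; Tick moves it along that facing by NewVar0 per frame, without delta time, and destroys it after about five seconds.
; Overlapping a BP_Enemy with RangeCollision applies truncated ProjectileDamage and destroys the projectile.
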(event `self.ReceiveBeginPlay`
  (bind _returnvalue (`GameplayStatics.GetPlayerCharacter` 0))
  (bind (_returnvalue_x _returnvalue_y _returnvalue_z) (`KismetMathLibrary.BreakVector` (`self.K2_GetActorLocation` _returnvalue)))
  (bind _yaw (.yaw (`self.K2_GetActorRotation` _returnvalue)))
  ;[1 1 1] Spawn the ranged attack in front of player
  (`self.K2_SetActorLocationAndRotation` (`KismetMathLibrary.MakeVector` (+ _returnvalue_x (* (`KismetMathLibrary.DegCos` _yaw) 80.0)) (+ _returnvalue_y (* (`KismetMathLibrary.DegSin` _yaw) 80.0)) _returnvalue_z) (`KismetMathLibrary.MakeRotator` (.roll (`self.K2_GetActorRotation` _returnvalue)) (.pitch (`self.K2_GetActorRotation` _returnvalue)) (+ _yaw -90.0))))

(event `self.ReceiveTick`
  (params (DeltaSeconds :type "Float (single-precision)"))
  (bind _newvar_0 (`self.NewVar_0`))
  (bind _yaw (.yaw (`self.K2_GetActorRotation`)))
  ;[1 1 1] Move the bullet forward
  (`self.K2_SetActorLocation` (`KismetMathLibrary.MakeVector` (+ (.x (`self.K2_GetActorLocation`)) (* (`KismetMathLibrary.DegSin` _yaw) (* -1.0 _newvar_0))) (+ (.y (`self.K2_GetActorLocation`)) (* (`KismetMathLibrary.DegCos` _yaw) _newvar_0)) (.z (`self.K2_GetActorLocation`))))
  ;[1 1 1] If ranged attack hasn't hit anything, destroy after ~5 seconds
  (`KismetSystemLibrary.Delay` 5.0)
  (`self.K2_DestroyActor`))

(event `self.Range Collision.OnComponentBeginOverlap`
  (params (OverlappedComponent :type "PrimitiveComponent Object Reference") (OtherActor :type "Actor Object Reference") (OtherComp :type "PrimitiveComponent Object Reference") (OtherBodyIndex :type Integer) (bFromSweep :type Boolean) (SweepResult :type "HitResult Structure (by ref)"))
  ;[1 1 1] Damage enemy hit
  (bind _asbp_enemy (cast `/Game/Enemies/BP_Enemy` OtherActor))
  (`/Game/Enemies/BP_Enemy.TakeDamage` _asbp_enemy (`KismetMathLibrary.FTrunc` (`self.projectile_damage`)))
  (`self.K2_DestroyActor`))

(fn `UserConstructionScript`)