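; BP_Ranged is a ranged attack projectile that damages enemies on contact.
; On BeginPlay it moves to the player character's X/Y at a fixed height and prints its location.
; Tick steps it along a fixed world-space diagonal, independent of player facing and not scaled by delta time.
; When RangedCollision overlaps a BP_Enemy, it calls that enemy's TakeDamage and destroys itself.
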(event `self.ReceiveBeginPlay`
  (`self.K2_SetActorLocation` (`KismetMathLibrary.MakeVector` (.x (`self.K2_GetActorLocation` (`GameplayStatics.GetPlayerCharacter` 0))) (.y (`self.K2_GetActorLocation` (`GameplayStatics.GetPlayerCharacter` 0))) 275.0))
  (`KismetSystemLibrary.PrintString` (`KismetStringLibrary.Conv_VectorToString` (`self.K2_GetActorLocation`))))

(event `self.RangedCollision.OnComponentBeginOverlap`
  (params (OverlappedComponent :type "PrimitiveComponent Object Reference") (OtherActor :type "Actor Object Reference") (OtherComp :type "PrimitiveComponent Object Reference") (OtherBodyIndex :type Integer) (bFromSweep :type Boolean) (SweepResult :type "HitResult Structure (by ref)"))
  (bind _asbp_enemy (cast `/Game/Enemies/BP_Enemy` OtherActor))
  (`/Game/Enemies/BP_Enemy.TakeDamage` _asbp_enemy 30)
  (`self.K2_DestroyActor`))

(event `self.ReceiveTick`
  (params (DeltaSeconds :type "Float (single-precision)"))
  (`self.K2_SetActorLocation` (`KismetMathLibrary.MakeVector` (+ (.x (`self.K2_GetActorLocation`)) 1.0) (+ (.y (`self.K2_GetActorLocation`)) 1.0) 275.0)))

(fn `UserConstructionScript`)