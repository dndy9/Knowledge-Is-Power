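; BP_EnemyAttack is an enemy bullet that deals a small amount of damage to the TopDownCharacter it overlaps, then destroys itself.
; Tick moves it a fixed step along its local right axis, computed from yaw with sine and cosine, without delta-time scaling.
; EnemyBulletLife counts down each tick and destroys the bullet at zero, so both speed and lifetime depend on frame rate.
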(event `self.ReceiveBeginPlay`)

(event `self.ReceiveActorBeginOverlap`
  (params (OtherActor :type "Actor Object Reference"))
  (bind _astop_down_character (cast `/Game/TopDownBP/Blueprints/TopDownCharacter` OtherActor))
  (`GameplayStatics.ApplyDamage` _astop_down_character 5.0)
  (`self.K2_DestroyActor`))

(event `self.ReceiveTick`
  (params (DeltaSeconds :type "Float (single-precision)"))
  (bind _yaw (.yaw (`self.K2_GetActorRotation`)))
  (`self.K2_SetActorLocation` (`KismetMathLibrary.MakeVector` (+ (.x (`self.K2_GetActorLocation`)) (* (`KismetMathLibrary.DegSin` _yaw) -2.5)) (+ (.y (`self.K2_GetActorLocation`)) (* (`KismetMathLibrary.DegCos` _yaw) 2.5)) (.z (`self.K2_GetActorLocation`))))
  (bind _result (`/Engine/EditorBlueprintResources/StandardMacros.DecrementInt` (`self.EnemyBulletLife`))
    (:`  `
      (if (<= _result 0)
        (`self.K2_DestroyActor`)))))

(fn `UserConstructionScript`)