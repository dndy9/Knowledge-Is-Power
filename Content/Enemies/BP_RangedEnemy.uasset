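; BP_RangedEnemy is an enemy actor that periodically spawns a BP_EnemyAttack at its own location.
; Tick decrements a WaitTimer counter each frame and fires when it drops below zero, so the cadence depends on frame rate.
; Each shot resets the counter to the sum of two random integers, varying the interval, and prints a debug string.
; The graph contains no targeting or movement logic.
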(event `self.ReceiveTick`
  (params (DeltaSeconds :type "Float (single-precision)"))
  (`parent.ReceiveTick` DeltaSeconds)
  (bind _result (`/Engine/EditorBlueprintResources/StandardMacros.DecrementInt` (`self.WaitTimer`))
    (:`  `
      (if (not (>= _result 0))
        (set `self.WaitTimer` (+ (`KismetMathLibrary.RandomInteger` 50) (`KismetMathLibrary.RandomInteger` 50)))
        (`KismetSystemLibrary.PrintString` "pew pew")
        (`|SpawnActorFromClass` "/Game/Enemies/BP_EnemyAttack.BP_EnemyAttack_C" (`KismetMathLibrary.MakeTransform` (`self.K2_GetActorLocation`)) "Undefined" "OverrideRootScale" null null)))))

(fn `UserConstructionScript`
  (`parent.UserConstructionScript`))