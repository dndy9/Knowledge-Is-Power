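; A quiz actor that shows a message widget while something overlaps its box trigger and hides it when the overlap ends.
; Overlap events toggle the HUDWidget component's hidden-in-game state without filtering the overlapping actor.
; SetQuizRef and GetQuizRef store and read a SQLite quiz widget reference on KIPGameInstance.
; A disconnected chain that would create that widget collapsed in the viewport and register it never runs.
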(event `self.ReceiveBeginPlay`)

(event `self.Box.OnComponentBeginOverlap`
  (params (OverlappedComponent :type "PrimitiveComponent Object Reference") (OtherActor :type "Actor Object Reference") (OtherComp :type "PrimitiveComponent Object Reference") (OtherBodyIndex :type Integer) (bFromSweep :type Boolean) (SweepResult :type "HitResult Structure (by ref)"))
  ;[1 1 1] step on the box to display message, step out to hide it
  (`SceneComponent.SetHiddenInGame` (`self.HUDWidget`) false false))

(event `self.Box.OnComponentEndOverlap`
  (params (OverlappedComponent :type "PrimitiveComponent Object Reference") (OtherActor :type "Actor Object Reference") (OtherComp :type "PrimitiveComponent Object Reference") (OtherBodyIndex :type Integer))
  ;[1 1 1] step on the box to display message, step out to hide it
  (`SceneComponent.SetHiddenInGame` (`self.HUDWidget`) true false))

(fn `getQuizRef`
  (returns (QuizRef :type "/Game/Quiz/Quiz-SQLite Object Reference"))
  (bind _askipgame_instance (cast `/Game/Blueprints/KIPGameInstance` (`GameplayStatics.GetGameInstance`)))
  (return (`/Game/Blueprints/KIPGameInstance.SQLiteWidgetRef` _askipgame_instance)))

(fn `setQuizRef`
  (params (QuizRef :type "/Game/Quiz/Quiz-SQLite Object Reference"))
  (bind _askipgame_instance (cast `/Game/Blueprints/KIPGameInstance` (`GameplayStatics.GetGameInstance`)))
  (set `/Game/Blueprints/KIPGameInstance.SQLiteWidgetRef` QuizRef _askipgame_instance))

(fn `UserConstructionScript`)