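; Enemy actor for a top-down game that homes in on the player and destroys itself when its health runs out.
; Tick moves it a small fraction of the remaining distance each frame, without delta-time scaling, and orients its Z axis away from the player.
; TakeDamage lowers and prints health, fed by collisions with TopDownCharacter and every tick while the AoEHit flag is set.
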(event `self.ReceiveTick`
  (params (DeltaSeconds :type "Float (single-precision)"))
  (bind _returnvalue (`self.K2_GetActorLocation`))
  (bind _returnvalue_2 (- _returnvalue (`self.K2_GetActorLocation` (`GameplayStatics.GetPlayerCharacter` 0))))
  ;[1 1 1] Update enemy position + where it's facing
  (`self.K2_SetActorLocationAndRotation` (- _returnvalue (* _returnvalue_2 0.0025)) (`KismetMathLibrary.MakeRotFromZ` _returnvalue_2))
  (if (`self.AoEHit`)
    (`self.TakeDamage` 3)))

(event `self.ReceiveBeginPlay`
  ;[1 1 1] Initialize enemy health
  (bind _output_get (set `self.EnemyHealth` 100))
  (`KismetSystemLibrary.PrintString` (`KismetStringLibrary.Conv_IntToString` _output_get)))

(event `self.ReceiveHit`
  (params (MyComp :type "PrimitiveComponent Object Reference") (Other :type "Actor Object Reference") (OtherComp :type "PrimitiveComponent Object Reference") (bSelfMoved :type Boolean) (HitLocation :type "Vector Structure") (HitNormal :type "Vector Structure") (NormalImpulse :type "Vector Structure") (Hit :type "HitResult Structure (by ref)"))
  ;[1 1 1] What happens when enemy is hit (for now it's only when the player runs into the enemy)
  (cast `/Game/TopDownBP/Blueprints/TopDownCharacter` Other)
  (`self.TakeDamage` 10))

(fn `TakeDamage`
  (params (Damage :type Integer))
  (bind _enemyhealth (`self.EnemyHealth`))
  (bind _output_get (set `self.EnemyHealth` (- _enemyhealth Damage)))
  (`KismetSystemLibrary.PrintString` (`KismetStringLibrary.Conv_IntToString` _output_get))
  (if (<= _enemyhealth 0)
    (`self.K2_DestroyActor`)))

(fn `UserConstructionScript`)